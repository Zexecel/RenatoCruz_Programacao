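; Enemy AI character that patrols a path or waits and looks around at a post, chasing the player on sight.
; Path and wait points become world locations at BeginPlay.
; Pawn sensing starts a looping chase timer, with a retriggerable delay detecting lost sight, and wait-type AIs alert all others to join.
; After losing the player, it searches random reachable points near the last target for a while, then resumes its previous state.
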(event `Wait`
  (bind (_returnvalue_roll _returnvalue_pitch _returnvalue_yaw) (`KismetMathLibrary.BreakRotator` (`self.K2_GetActorRotation`)))
  ;[0.1 0.1 0.1 1 25] WAIT STATE - move to desired wait location, then rotate the ai - make it look around
  (`KismetSystemLibrary.PrintString` "wait")
  (`|AIMoveTo` self (`self.WaitLocation`) null 25.0
    (:`OnSuccess`
      (if (and (not (`self.Can see player`)) (`|EnumEquality` (`self.State`) "NewEnumerator1")) :!label _label
        (set `self.RandomRotation` (/ (`KismetMathLibrary.RandomFloatInRange` 0.0 360.0) 2.0))
        (set `self.CurrentRotation` _returnvalue_yaw)
        (bind (_direction _newtrack_0) (`Timeline|Timeline_0` :!via `PlayFromStart`)
          (:`Update`
            (`self.K2_SetActorRotation` (`KismetMathLibrary.MakeRotator` 0.0 0.0 (`KismetMathLibrary.Lerp` (`self.CurrentRotation`) (`self.RandomRotation`) _newtrack_0))))
          (:`Finished`
            (`KismetSystemLibrary.Delay` (`KismetMathLibrary.RandomFloatInRange` 2.0 5.0))
            (goto _label)))))))

(event `self.ReceiveBeginPlay`
  (bind _returnvalue (`self.GetTransform`))
  (bind _path (`self.Path`))
  ;[0.1 0.1 0.1 1 25] Beginplay called at the start of the game. Set timer for changing states, then initiate the corresponding state. Change locations from relative to world
  (for (_array_element _array_index) _path
    (`KismetArrayLibrary.Array_Set` _path _array_index (`KismetMathLibrary.TransformLocation` _returnvalue _array_element)))
  (set `self.WaitLocation` (`KismetMathLibrary.TransformLocation` _returnvalue (`self.WaitLocation`)))
  (set `self.PrevState` (`self.State`))
  (switch `/Game/Blueprints/AI/E_AIState` (`self.State`)
    (:`NewEnumerator0`
      (`self.Patrol`))
    (:`NewEnumerator1`
      (`self.Wait`))))

(event `self.PawnSensing.OnSeePawn`
  (params (Pawn :type "Pawn Object Reference"))
  ;[0.1042 0.1042 0.1042 1 25] On See Pawn - when enemy sees the player - initiate chase state, stop any other actions from previous state, set current state to chase, set it to call the chase event every 0.05 seconds
  (cast `PlayerCharacter` Pawn)
  (`|ExecutionSequence`
    (:`then_0`
      (set `self.Can see player` true :!label _label_2)
      (`/Engine/EditorBlueprintResources/StandardMacros.DoOnce` false :!label _label_3
        (:`Completed`
          (`self.BroadcastPlayerLocation`)
          (`self.Chase player`)
          (`MovementComponent.StopMovementImmediately` (`self.CharacterMovement`))
          (`TimelineComponent.Stop` (`self.Timeline_0`))
          (set `self.State` "NewEnumerator2")
          (`KismetSystemLibrary.K2_SetTimer` null "Chase player" 0.05 true)
          (goto _label_5 :!via `Reset`))))
    (:`then_1`
      (`KismetSystemLibrary.RetriggerableDelay` 0.4 :!label _label_4)
      (set `self.Can see player` false)
      (`/Engine/EditorBlueprintResources/StandardMacros.DoOnce` true :!label _label_5
        (:`Completed`
          (`KismetSystemLibrary.K2_ClearTimer` null "Chase player")
          (goto _label_3 :!via `Reset`))))))

(event `Patrol`
  (bind _pathindex (`self.PathIndex`))
  ;[0.1 0.1 0.1 1 25] PATROL STATE - get path location at index, move to that location.
  (set `CharacterMovementComponent.MaxWalkSpeed` 200.0 (`self.CharacterMovement`))
  (set `self.TargetLocation` (`|GetArrayItem` (`self.Path`) (`self.PathIndex`)))
  (`|AIMoveTo` self (`self.TargetLocation`) null 25.0
    (:`OnSuccess`
      (`KismetSystemLibrary.Delay` (`KismetMathLibrary.RandomFloatInRange` 2.0 6.0))
      (if (`|EnumEquality` (`self.State`) "NewEnumerator0")
        (`/Engine/EditorBlueprintResources/StandardMacros.IncrementInt` _pathindex
          (:`  `
            (set `self.PathIndex` (mod _pathindex (`KismetArrayLibrary.Array_Length` (`self.Path`))))
            (`self.Patrol`)))))))

(event `StartChasing`
  ;[0.1042 0.1042 0.1042 1 25] On See Pawn - when enemy sees the player - initiate chase state, stop any other actions from previous state, set current state to chase, set it to call the chase event every 0.05 seconds
  (if (not (`self.Can see player`))
    (`|ExecutionSequence`
      (:`then_0`
        (goto _label_2))
      (:`then_1`
        (`KismetSystemLibrary.Delay` 3.0)
        (goto _label_4)))))

(event `BroadcastPlayerLocation`
  ;[0.1042 0.1042 0.1042 1 25] Broadcast the player location to other ais if this is the wait ai
  (if (`|EnumEquality` (`self.PrevState`) "NewEnumerator1")
    (bind _outactors (`GameplayStatics.GetAllActorsOfClass` "BP_AICharacter_C"))
    (for _array_element _outactors
      (if (!= _array_element self)
        (`self.StartChasing` _array_element)))))

(event `Chase player`
  ;[0.1042 0.1042 0.1042 1 25] CHASE STATE - set the target player location, increase walking speed, move to the target location. When finished moving to location and the sight of player is lost - for 30 seconds move to random locations around the players location and set state to the pre chase state and initiate it accordingly
  (set `self.TargetLocation` (`self.K2_GetActorLocation` (`GameplayStatics.GetPlayerCharacter` 0)))
  (set `CharacterMovementComponent.MaxWalkSpeed` 400.0 (`self.CharacterMovement`))
  (`|AIMoveTo` self (`self.TargetLocation`) null 25.0
    (:`OnSuccess`
      _)
    (:`OnFail`
      _))
  (if (not (`self.Can see player`))
    (`|ExecutionSequence`
      (:`then_0`
        (goto _label_7 :!via `Reset`))
      (:`then_1`
        (if (`|EnumInequality` (`self.State`) (`self.PrevState`)) :!label _label_6
          (`|AIMoveTo` self (`NavigationSystemV1.K2_GetRandomReachablePointInRadius` (`self.TargetLocation`) 250.0 null null) null 10.0
            (:`then`
              (`/Engine/EditorBlueprintResources/StandardMacros.DoOnce` false :!label _label_7
                (:`Completed`
                  (`KismetSystemLibrary.RetriggerableDelay` 30.0)
                  (bind _output_get (set `self.State` (`self.PrevState`)))
                  (switch `/Game/Blueprints/AI/E_AIState` _output_get
                    (:`NewEnumerator0`
                      (`self.Patrol`))
                    (:`NewEnumerator1`
                      (`self.Wait`))))))
            (:`OnSuccess`
              (`KismetSystemLibrary.Delay` (`KismetMathLibrary.RandomFloatInRange` 1.0 2.0))
              (goto _label_6))))))))

(fn `UserConstructionScript`)